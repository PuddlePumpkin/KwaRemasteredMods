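; Example actor for the Kwa notifications mod, demonstrating how to use BP_NotificationComponent.
; When the component is ready, it prints normal and debug notifications, enables debug messages, and calls the slower global library function.
; A debug key on T prints a test notification.
; Handlers for the component's any, Kwa and vanilla notification events echo each message with PrintString.
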(event OnReady(BP_NotificationComponent)
  ;[1 1 1] Created  by clicking the notification component, scrolling down to events
  ;[1 1 1] Print a notif
  (Default|PrintNotification (Variables|Default|GetBP_NotificationComponent) "ON READY FIRED" 5.0)
  ;[1 1 1] print a notif if debug is enabled (its not so this does nothing)
  (Default|PrintNotificationDebug (Variables|Default|GetBP_NotificationComponent) "This Shouldnt Show Up" 7.0)
  ;[1 1 1] enable debug
  (Default|SetDebugMessagesEnabled (Variables|Default|GetBP_NotificationComponent) true)
  ;[1 1 1] now a debug notif comes up (this shows every kwa integrated mod's debug notifications)
  (Default|PrintNotificationDebug (Variables|Default|GetBP_NotificationComponent) "This Should Show Up" 8.0)
  ;[1 1 1] this is a call to the global function library, it uses get all widgets of class so should be used sparingly
  (CallFunction|PrintNotificationSlow "Global notification function (but slow)" 9.0))

(event OnAnyNotification(BP_NotificationComponent)
  (params (String :type String) (Duration :type Float%20%28double-precision%29) (Texture :type Texture%202D%20Object%20Reference))
  ;[1 1 1] Additional Events
  (Development|PrintString (Utilities|String|Append "Any Notification Fired: " String)))

(event OnKwaNotification(BP_NotificationComponent)
  (params (String :type String) (Duration :type Float%20%28double-precision%29) (Texture :type Texture%202D%20Object%20Reference))
  ;[1 1 1] Additional Events
  (Development|PrintString (Utilities|String|Append "Notification Fired From Helper Functions: " String)))

(event OnVanillaNotification(BP_NotificationComponent)
  (params (Properties :type Legacy%20Notification%20Properties%20Structure) (String :type String))
  ;[1 1 1] Additional Events
  (Development|PrintString (Utilities|String|Append "Vanilla Notification Fired: " String)))

(event Input|KeyboardEvents|DebugKeyT
  (params (Key :type Key%20Structure :default "None") (ActionValue :type Input%20Action%20Value%20Structure))
  ;[1 1 1] Debug keys are called in editor but are left out of being packaged
  (:Pressed
    (Default|PrintNotification (Variables|Default|GetBP_NotificationComponent) "This is a test of the component system" 3.0)))

(fn ConstructionScript)