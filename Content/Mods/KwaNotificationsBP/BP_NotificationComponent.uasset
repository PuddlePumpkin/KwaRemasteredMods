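; Actor component that gives access to the KwaNotifications widget (WBP_KwaNotifs) for printing on-screen notifications and listening to them.
; BeginPlay finds the top-level widget and fires OnReady; Tick retries while it is invalid, then binds its events and disables itself.
; Vanilla, Kwa and Any notification events are re-broadcast through the component's dispatchers.
; Functions forward plain, icon and debug prints, plus the debug-message toggle, to the widget when valid.
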(event `PassthroughNotifVanilla`
  (params (Properties :type "LegacyNotificationProperties Structure") (String :type String))
  ;[0 0 0] Passthrough Event Bindings
  (`self.OnVanillaNotification` Properties String))

(event `PassthroughNotifKwa`
  (params (String :type String) (Duration :type "Float (double-precision)") (Texture :type "Texture2D Object Reference"))
  ;[0 0 0] Passthrough Event Bindings
  (`self.OnKwaNotification` String Duration Texture))

(event `PassthroughNotifAny`
  (params (String :type String) (Duration :type "Float (double-precision)") (Texture :type "Texture2D Object Reference"))
  ;[0 0 0] Passthrough Event Bindings
  (`self.OnAnyNotification` String Duration Texture))

(event `self.ReceiveBeginPlay`
  ;[0 0 0] Find Notification Widget
  (bind _foundwidgets (`WidgetBlueprintLibrary.GetAllWidgetsOfClass` "/Game/Mods/KwaNotificationsBP/WBP_KwaNotifs.WBP_KwaNotifs_C"))
  (set `self.EntryPointReference` (`|GetArrayItem` _foundwidgets))
  (set `self.Ready` true)
  (`self.OnReady`))

(event `self.ReceiveTick`
  (params (DeltaSeconds :type "Float (single-precision)"))
  (bind _entrypointreference (`self.EntryPointReference`))
  ;[0 0 0] Find Notification Widget
  ;;[1 0.1674 0.9764] Tick (set to 1 second ticks)
  (`/Engine/EditorBlueprintResources/StandardMacros.IsValid` _entrypointreference
    (:`Is Valid`
      (add `/Game/Mods/KwaNotificationsBP/WBP_KwaNotifs.OnVanillaNotification` _entrypointreference (delegate `PassthroughNotifVanilla`))
      (add `/Game/Mods/KwaNotificationsBP/WBP_KwaNotifs.OnKwaNotification` _entrypointreference (delegate `PassthroughNotifKwa`))
      (add `/Game/Mods/KwaNotificationsBP/WBP_KwaNotifs.OnAnyNotification` _entrypointreference (delegate `PassthroughNotifAny`))
      (`self.SetComponentTickEnabled` false))
    (:`Is Not Valid`
      (bind _foundwidgets (`WidgetBlueprintLibrary.GetAllWidgetsOfClass` "/Game/Mods/KwaNotificationsBP/WBP_KwaNotifs.WBP_KwaNotifs_C"))
      (set `self.EntryPointReference` (`|GetArrayItem` _foundwidgets))
      (set `self.Ready` true)
      (`self.OnReady`))))

(fn `PrintNotification`
  (params (String :type String) (Duration :type "Float (double-precision)" :default 3.0))
  (bind _entrypointreference (`self.EntryPointReference`))
  (if (`self.Ready`)
    (`/Engine/EditorBlueprintResources/StandardMacros.IsValid` _entrypointreference
      (:`Is Valid`
        (`/Game/Mods/KwaNotificationsBP/WBP_KwaNotifs.PrintNotification` _entrypointreference String Duration)))))

(fn `PrintNotificationDebug`
  (params (String :type String) (Duration :type "Float (double-precision)" :default 3.0) (Texture :type "Texture2D Object Reference"))
  (bind _entrypointreference (`self.EntryPointReference`))
  (if (`self.Ready`)
    (`/Engine/EditorBlueprintResources/StandardMacros.IsValid` _entrypointreference
      (:`Is Valid`
        (`/Game/Mods/KwaNotificationsBP/WBP_KwaNotifs.PrintNotificationDebug` _entrypointreference String Duration Texture)))))

(fn `PrintNotificationWithIcon`
  (params (String :type String) (Duration :type "Float (double-precision)" :default 3.0) (Texture :type "Texture2D Object Reference"))
  (bind _entrypointreference (`self.EntryPointReference`))
  (if (`self.Ready`)
    (`/Engine/EditorBlueprintResources/StandardMacros.IsValid` _entrypointreference
      (:`Is Valid`
        (`/Game/Mods/KwaNotificationsBP/WBP_KwaNotifs.PrintNotificationWithIcon` _entrypointreference String Duration Texture)))))

(fn `SetDebugMessagesEnabled`
  (params (Enabled :type Boolean))
  (bind _entrypointreference (`self.EntryPointReference`))
  (`/Engine/EditorBlueprintResources/StandardMacros.IsValid` _entrypointreference
    (:`Is Valid`
      (`/Game/Mods/KwaNotificationsBP/WBP_KwaNotifs.SetDebugMessagesEnabled` _entrypointreference Enabled))))